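; BP_A1 is an AI-driven asteroid that takes damage when hit.
; On BeginPlay its AI controller runs the A1_AI_BT behavior tree.
; Each hit briefly swaps the mesh material, plays a damage sound, then subtracts a fixed amount of health after the delay.
; Health is checked before subtraction, so the asteroid is destroyed only by a hit that arrives once health is already depleted.
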(event Collision|EventHit
  (params (MyComp :type Primitive%20Component%20Object%20Reference) (Other :type Actor%20Object%20Reference) (OtherComp :type Primitive%20Component%20Object%20Reference) (bSelfMoved :type Boolean) (HitLocation :type Vector :default "0, 0, 0") (HitNormal :type Vector :default "0, 0, 0") (NormalImpulse :type Vector :default "0, 0, 0") (Hit :type Hit%20Result%20Structure%20%28by%20ref%29))
  (if (<= (Variables|Default|GetAsteroidHealth) 0.0)
    (Actor|DestroyActor)
    (else
      (Rendering|Material|SetMaterial (Variables|Character|GetMesh) 0 "/Game/Game_Objects/Asteroids/A5/M_A5.M_A5")
      (Audio|PlaySound2D "/Game/Game_Objects/Audio/AstroidsSFX/AstroDamaged1.AstroDamaged1" 1.0 1.0 0.0 0 0)
      (Utilities|FlowControl|Delay 0.3)
      (Rendering|Material|SetMaterial (Variables|Character|GetMesh) 0 "/Game/Game_Objects/Asteroids/A1/M_A1.M_A1")
      (Variables|Default|SetAsteroidHealth (- (Variables|Default|GetAsteroidHealth) 5e+01)))))

(event EventBeginPlay
  (AI|RunBehaviorTree (AI|GetAIController self) "/Game/Game_Objects/Asteroids/A1/A1_AI_BT.A1_AI_BT"))

(fn ConstructionScript)