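; Earth actor for a VR game that takes damage from asteroid impacts and registers itself with VRGameMode.
; Overlaps briefly flash a hit material and pick one of five damage tiers from the asteroid's display-name prefix.
; Tiers destroy the asteroid and lower the health widget's progress bar, which holds Earth's health.
; A5 empties it and triggers EarthDestroyed after a delay, hiding the HUD; otherwise destruction waits for an overlap at zero health.
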(event EventBeginPlay
  ;[1 1 1] Begin PLay
  (bind _asearth_health_bar (Utilities|Casting|CastToEarthHealthBar (UserInterface|GetUserWidgetObject (Variables|Default|GetHealthBar))))
  (Variables|Default|SetEarthHealthBarRef _asearth_health_bar)
  (bind _asvrgame_mode (Utilities|Casting|CastToVRGameMode (Game|GetGameMode)))
  (Variables|/Game/VRTemplate/Blueprints/VRGameMode.VRGameMode_C|SetBP_Earth _asvrgame_mode self)
  (Variables|Default|SetEarthHealthPercent (Variables|/Script/UMG.ProgressBar|GetPercent (Variables|/Game/Game_Objects/Earth/EarthHealthBar.EarthHealthBar_C|GetProgressBar_56 (Variables|Default|GetEarthHealthBarRef)))))

(event Collision|EventActorBeginOverlap
  (params (OtherActor :type Actor%20Object%20Reference))
  ;[0.3294 1 0.9302] Asteroid Hit Detection
  (if (<= (Variables|Default|GetEarthHealthPercent) 0.0)
    (Utilities|FlowControl|DoOnce false
      (:Completed
        (CallFunction|EarthDestroyed)))
    (else
      (Rendering|Material|SetMaterial (Variables|Default|GetEarth) 0 "/Game/Game_Objects/Earth/Earth_MATERIAL_HIT.Earth_MATERIAL_HIT")
      (Utilities|FlowControl|Delay 0.5)
      (Rendering|Material|SetMaterial (Variables|Default|GetEarth) 0 "/Game/Game_Objects/Earth/Earth_MATERIAL.Earth_MATERIAL")
      (bind _output_get (Variables|Default|SetAsteroidActor OtherActor))
      (switch string (Utilities|String|GetSubstring (Utilities|GetDisplayName OtherActor) 0 5)
        (:BP_A1
          (CallFunction|A1Hit _output_get))
        (:BP_A2
          (CallFunction|A2Hit _output_get))
        (:BP_A3
          (CallFunction|A3Hit _output_get))
        (:BP_A4
          (CallFunction|A4Hit _output_get))
        (:BP_A5
          (CallFunction|A5Hit _output_get)
          (Utilities|FlowControl|Delay 2.0)
          (CallFunction|EarthDestroyed))))))

(fn ConstructionScript)

(fn A1Hit
  (params (Asteroid :type Actor%20Object%20Reference))
  (bind _earthhealthbarref (Variables|Default|GetEarthHealthBarRef))
  (bind _progressbar_56 (Variables|/Game/Game_Objects/Earth/EarthHealthBar.EarthHealthBar_C|GetProgressBar_56 _earthhealthbarref))
  (Actor|DestroyActor Asteroid)
  (bind _output_get (Variables|Default|SetEarthHealthPercent (- (Variables|/Script/UMG.ProgressBar|GetPercent _progressbar_56) 0.01)))
  (Progress|SetPercent _progressbar_56 _output_get)
  (Development|PrintString "A1 Hit!" true true "(R=1.000000,G=1.000000,B=1.000000,A=1.000000)" 5.0))

(fn A2Hit
  (params (Asteroid :type Actor%20Object%20Reference))
  (bind _earthhealthbarref (Variables|Default|GetEarthHealthBarRef))
  (bind _progressbar_56 (Variables|/Game/Game_Objects/Earth/EarthHealthBar.EarthHealthBar_C|GetProgressBar_56 _earthhealthbarref))
  (Actor|DestroyActor Asteroid)
  (bind _output_get (Variables|Default|SetEarthHealthPercent (- (Variables|/Script/UMG.ProgressBar|GetPercent _progressbar_56) 0.03)))
  (Progress|SetPercent _progressbar_56 _output_get)
  (Development|PrintString "A2 Hit!" true true "(R=0.000000,G=0.271455,B=1.000000,A=1.000000)" 5.0))

(fn A3Hit
  (params (Asteroid :type Actor%20Object%20Reference))
  (bind _earthhealthbarref (Variables|Default|GetEarthHealthBarRef))
  (bind _progressbar_56 (Variables|/Game/Game_Objects/Earth/EarthHealthBar.EarthHealthBar_C|GetProgressBar_56 _earthhealthbarref))
  (Actor|DestroyActor Asteroid)
  (bind _output_get (Variables|Default|SetEarthHealthPercent (- (Variables|/Script/UMG.ProgressBar|GetPercent _progressbar_56) 0.1)))
  (Progress|SetPercent _progressbar_56 _output_get)
  (Development|PrintString "A3 Hit!" true true "(R=1.000000,G=0.991496,B=0.000000,A=1.000000)" 5.0))

(fn A4Hit
  (params (Asteroid :type Actor%20Object%20Reference))
  (bind _earthhealthbarref (Variables|Default|GetEarthHealthBarRef))
  (bind _progressbar_56 (Variables|/Game/Game_Objects/Earth/EarthHealthBar.EarthHealthBar_C|GetProgressBar_56 _earthhealthbarref))
  (Actor|DestroyActor Asteroid)
  (bind _output_get (Variables|Default|SetEarthHealthPercent (- (Variables|/Script/UMG.ProgressBar|GetPercent _progressbar_56) 0.25)))
  (Progress|SetPercent _progressbar_56 _output_get)
  (Default|CallEarthHit _output_get))

(fn A5Hit
  (params (Asteroid :type Actor%20Object%20Reference))
  (Actor|DestroyActor Asteroid)
  (bind _output_get (Variables|Default|SetEarthHealthPercent 0.0))
  (Progress|SetPercent (Variables|/Game/Game_Objects/Earth/EarthHealthBar.EarthHealthBar_C|GetProgressBar_56 (Variables|Default|GetEarthHealthBarRef)) _output_get)
  (Default|CallEarthHit 0.0))

(fn EarthDestroyed
  (Rendering|Material|SetMaterial (Variables|Default|GetEarth) 0 "/Game/Game_Objects/Earth/Earth_MATERIAL_HIT.Earth_MATERIAL_HIT")
  (bind _asvrgame_mode (Utilities|Casting|CastToVRGameMode (Game|GetGameMode)))
  (Widget|SetVisibility (UserInterface|GetWidget (Variables|/Game/VRTemplate/Blueprints/VRPawn.VRPawn_C|GetWidgetHUD (Variables|/Game/VRTemplate/Blueprints/VRGameMode.VRGameMode_C|GetVRPawn _asvrgame_mode))) "Hidden")
  (Game|SetGamePaused false))